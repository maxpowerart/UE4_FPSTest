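; BP_BoxDamageArea is a box-shaped area that periodically damages any FPSCharacterBase inside it through the Gameplay Ability System.
; A looping one-second timer started on BeginPlay polls the box's overlapping actors, with damage applied only on the server.
; Each character's own ability system component builds and self-applies the configurable damage effect, passing Damage as a Data.Damage SetByCaller magnitude.
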(event Custom|DamageTick
  (Networking|SwitchHasAuthority
    (:Authority
      (for _array_element (Collision|GetOverlappingActors (Variables|Default|GetBox) 0 :!class /Script/Engine.PrimitiveComponent)
        (bind _asfpscharacter_base (Utilities|Casting|CastToFPSCharacterBase _array_element))
        (if (and true (Utilities|IsValid (Ability|GetAbilitySystemComponent _asfpscharacter_base)))
          (bind _returnvalue (Ability|GameplayEffect|AssignTagSetbyCallerMagnitude (GameplayEffects|MakeOutgoingSpec (Ability|GetAbilitySystemComponent _asfpscharacter_base) (Variables|Default|GetDamageGameplayEffectClass) 1.0 (GameplayEffects|MakeEffectContext (Ability|GetAbilitySystemComponent _asfpscharacter_base))) "(TagName=\"Data.Damage\")" (Variables|Default|GetDamage)))
          (GameplayEffects|ApplyGameplayEffectSpecToSelf (Ability|GetAbilitySystemComponent _asfpscharacter_base) _returnvalue))))))

(event EventBeginPlay
  (Utilities|Time|SetTimerbyEvent (delegate Custom|DamageTick) 1.0 true))

(fn ConstructionScript)